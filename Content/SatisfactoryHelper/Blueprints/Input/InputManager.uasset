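; InputManager is an actor in the SatisfactoryHelper mod that handles the hotkey for the items window.
; On BeginPlay it caches the local FGPlayerController, logging a fatal error if the cast fails.
; Each Tick it polls the toggle key and toggles the ItemsWidget through InitMod's UIManager.
; If the widget starts fading, it matches the mouse cursor and virtual cursor to the widget's visibility.
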(event EventBeginPlay
  (bind _asfgplayer_controller (Utilities|Casting|CastToFGPlayerController (Game|GetPlayerController 0))
    (:then
      (Variables|Default|SetPlayerController _asfgplayer_controller))
    (:CastFailed
      (Class|SMLBlueprintLibrary|LogFatal "Could not cast player controller to FGPlayerController"))))

(event EventTick
  (params (DeltaSeconds :type Float%20%28single-precision%29))
  (bind _playercontroller (Variables|Default|GetPlayerController))
  (if (Game|Player|WasInputKeyJustPressed (Variables|Default|GetPlayerController) (Variables|Default|GetToggleItemsWindowKey))
    (bind (_isfading _isvisible) (Default|ToggleWidget (Variables|/Game/SatisfactoryHelper/Blueprints/UI/UIManager.UIManager_C|GetItemsWidget (Variables|/Game/SatisfactoryHelper/InitMod.InitMod_C|GetUIManager (Variables|Default|GetInitMod)))))
    (if _isfading
      (bind _output_get (Variables|/Script/Engine.PlayerController|SetbShowMouseCursor _playercontroller _isvisible))
      (if _output_get
        (Class|FGVirtualCursorFunctionLibrary|EnableVirtualCursor _playercontroller)
        (else
          (Class|FGVirtualCursorFunctionLibrary|DisableVirtualCursor _playercontroller))))))

(fn ConstructionScript)